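; BP_EnemyManager is an enemy spawner that repeatedly creates BP_Enemy actors at its own transform.
; BeginPlay starts a looping timer by function name that calls CreateEnemy every CreateTime interval.
; An alternative elapsed-time accumulator that would call the same function is left unconnected, and Tick does nothing.
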(event `self.ReceiveBeginPlay`
  ;[1 1 1] 밑의 노드를 이 노드로 요약가능
  (`KismetSystemLibrary.K2_SetTimer` null "CreateEnemy" (`self.CreateTime`) true))

(event `self.ReceiveTick`
  (params (DeltaSeconds :type "Float (single-precision)"))
  ;[1 1 1] 현재시간이 경과시간 이상이 된다면
)

(fn `CreateEnemy`
  (`|SpawnActorFromClass` "/Game/BluePrints/BP_Enemy.BP_Enemy_C" (`self.GetTransform`) "Undefined" "OverrideRootScale" null null))

(fn `UserConstructionScript`)