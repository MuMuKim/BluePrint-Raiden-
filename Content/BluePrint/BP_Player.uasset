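; BP_Player is a player actor that moves in the Y/Z plane from horizontal and vertical input.
; On BeginPlay it enables input from the first player controller.
; Each Tick it normalizes the input vector, scales it by Speed and delta seconds, and offsets the actor location without sweeping, so diagonal movement is no faster and blocking collision does not stop it.
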(event `self.ReceiveBeginPlay`
  ;[1 1 1] Actor 입력활성화
  (`self.EnableInput` (`GameplayStatics.GetPlayerController` 0)))

(event `self.ReceiveTick`
  (params (DeltaSeconds :type "Float (single-precision)"))
  (`self.K2_SetActorLocation` (+ (* (* (`KismetMathLibrary.Normal` (`KismetMathLibrary.MakeVector` 0.0 (`self.GetInputAxisValue`) (`self.GetInputAxisValue`))) (`self.Speed`)) DeltaSeconds) (`self.K2_GetActorLocation`))))

(fn `UserConstructionScript`)